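; PC_Cannon handles Left and Right key input to step the Ship_BP actor sideways along the world Y axis.
; Each press looks up the ship with GetActorOfClass and sets its location one fixed step over, keeping X and Z.
; A step that would pass the lane limit negates the current Y instead, wrapping the ship to the opposite side.
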(event `Key|Left`
  (params (Key :type "Key Structure"))
  (:`Pressed`
    (bind _returnvalue (`GameplayStatics.GetActorOfClass` "/Game/Blueprints/Ship_BP.Ship_BP_C"))
    (bind (_returnvalue_x _returnvalue_y _returnvalue_z) (`KismetMathLibrary.BreakVector` (`self.K2_GetActorLocation` _returnvalue)))
    (bind _returnvalue_2 (- _returnvalue_y 1000.0))
    (if (< _returnvalue_2 -4000.0)
      (`self.K2_SetActorLocation` _returnvalue (`KismetMathLibrary.MakeVector` _returnvalue_x (* -1 _returnvalue_y) _returnvalue_z) false false)
      (else
        (`self.K2_SetActorLocation` _returnvalue (`KismetMathLibrary.MakeVector` _returnvalue_x _returnvalue_2 _returnvalue_z) false false)))))

(event `Key|Right`
  (params (Key :type "Key Structure"))
  (:`Pressed`
    (bind _returnvalue (`GameplayStatics.GetActorOfClass` "/Game/Blueprints/Ship_BP.Ship_BP_C"))
    (bind (_returnvalue_x _returnvalue_y _returnvalue_z) (`KismetMathLibrary.BreakVector` (`self.K2_GetActorLocation` _returnvalue)))
    (bind _returnvalue_2 (+ _returnvalue_y 1000.0))
    (if (> _returnvalue_2 4000.0)
      (`self.K2_SetActorLocation` _returnvalue (`KismetMathLibrary.MakeVector` _returnvalue_x (* -1 _returnvalue_y) _returnvalue_z) false false)
      (else
        (`self.K2_SetActorLocation` _returnvalue (`KismetMathLibrary.MakeVector` _returnvalue_x _returnvalue_2 _returnvalue_z) false false)))))

(fn `UserConstructionScript`)