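; Ship actor that fakes moving closer to the camera by scaling itself up while lowering its Z position.
; Tick runs through a Delay to apply each step until the relative Y scale reaches its cap.
; Despite its name, RandomValue is a fixed countdown set on BeginPlay, which shrinks the scale increment and enlarges the drop over the first few steps.
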(event `self.ReceiveBeginPlay`
  ;[1 1 1] Set Random Value to 2
  (set `self.RandomValue` 3))

(event `self.ReceiveTick`
  (params (DeltaSeconds :type "Float (single-precision)"))
  (bind (_returnvalue_x _returnvalue_y _returnvalue_z) (`KismetMathLibrary.BreakVector` (`self.GetActorRelativeScale3D`)))
  (bind (_returnvalue_x_2 _returnvalue_y_2 _returnvalue_z_2) (`KismetMathLibrary.BreakVector` (`self.K2_GetActorLocation`)))
  (bind _scalevalue (`self.ScaleValue`))
  (bind _randomvalue (`self.RandomValue`))
  ;[1 1 1] Move Closer To Camera
  (`KismetSystemLibrary.Delay` (`self.DelaySpeed`))
  (if (< _returnvalue_y 2.4)
    (`self.SetActorRelativeScale3D` (`KismetMathLibrary.MakeVector` (+ _returnvalue_x _scalevalue) (+ _returnvalue_y _scalevalue) (+ _returnvalue_z _scalevalue)))
    (`self.K2_SetActorLocation` (`KismetMathLibrary.MakeVector` _returnvalue_x_2 _returnvalue_y_2 (- _returnvalue_z_2 (`self.ActorLocationValue`))))
    (if (not (== _randomvalue 0))
      (set `self.RandomValue` (- _randomvalue 1))
      (if (<= (`self.RandomValue`) 2)
        (set `self.ScaleValue` (- (`self.ScaleValue`) 0.05))
        (set `self.ActorLocationValue` (+ (`self.ActorLocationValue`) 10.0))))))

(fn `UserConstructionScript`)