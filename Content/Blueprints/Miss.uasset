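; Miss Blueprint that briefly flashes a miss indicator, alternating between a left and a right component.
; The RenderMisses event checks the Left boolean, shows MissLeft or MissRight, then hides it after a short delay.
; Left flips only after that delay completes, so the next call after it uses the opposite side.
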(event `RenderMisses`
  (bind _missleft (`self.MissLeft`))
  (bind _missright (`self.MissRight`))
  (if (`self.Left`)
    (`SceneComponent.SetVisibility` _missleft true false)
    (`KismetSystemLibrary.Delay` 0.3)
    (`SceneComponent.SetVisibility` _missleft false false)
    (set `self.Left` false)
    (else
      (`SceneComponent.SetVisibility` _missright true false)
      (`KismetSystemLibrary.Delay` 0.3)
      (`SceneComponent.SetVisibility` _missright false false)
      (set `self.Left` true))))

(fn `UserConstructionScript`)